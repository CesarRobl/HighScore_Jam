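; Shop actor that offers a shop screen while the shark player is within its trigger box.
; BeginPlay creates the shop widget once and caches the level's upgrade manager.
; Box overlaps with the shark player toggle an in-range flag.
; The ShopUI function checks that flag, then fills in item info and adds the widget to the viewport; the ShowShopUI event is an empty stub.
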(event OnComponentBeginOverlap(Box)
  (params (OverlappedComponent :type Primitive%20Component%20Object%20Reference) (OtherActor :type Actor%20Object%20Reference) (OtherComp :type Primitive%20Component%20Object%20Reference) (OtherBodyIndex :type Integer) (bFromSweep :type Boolean) (SweepResult :type Hit%20Result%20Structure%20%28by%20ref%29))
  (Utilities|Casting|CastToBP_SharkPlayer OtherActor)
  (Variables|Default|SetInRange true))

(event OnComponentEndOverlap(Box)
  (params (OverlappedComponent :type Primitive%20Component%20Object%20Reference) (OtherActor :type Actor%20Object%20Reference) (OtherComp :type Primitive%20Component%20Object%20Reference) (OtherBodyIndex :type Integer))
  (Utilities|Casting|CastToBP_SharkPlayer OtherActor)
  (Variables|Default|SetInRange false))

(event EventBeginPlay
  (bind _returnvalue (UserInterface|CreateWidget "/Game/Blueprints/Widgets/BP_ShopUI.BP_ShopUI_C" (Game|GetPlayerController 0)))
  (Variables|Default|SetShopUI _returnvalue)
  (bind _returnvalue_2 (Actor|GetActorOfClass "/Game/Blueprints/Actors/Managers/BP_UpgradeManager.BP_UpgradeManager_C"))
  (Variables|Default|SetUpgrade%20Manager _returnvalue_2))

(event Collision|EventActorBeginOverlap
  (params (OtherActor :type Actor%20Object%20Reference)))

(event EventTick
  (params (DeltaSeconds :type Float%20%28single-precision%29)))

(event EventShowShopUI)

(fn ConstructionScript)

(fn ShopUI
  (bind _shopui (Variables|Default|GetShopUI))
  (if (Variables|Default|GetInRange)
    (Default|AddShopItemInfo _shopui)
    (UserInterface|Viewport|AddtoViewport _shopui 0)))