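; BP_EventManager is an actor that starts game events and handles their UI.
; After a short delay on BeginPlay, it caches the first player controller as a ScorePlayerController and calls SpawnEvent, which is not defined in these graphs.
; ShowRewardsUI creates the BP_EventRewards widget, adds it to the viewport and shows the mouse cursor.
; SwitchEventUI toggles the visibility of the event timer in the player UI.
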(event EventBeginPlay
  (Utilities|FlowControl|Delay 0.3)
  (bind _asscore_player_controller (Utilities|Casting|CastToScorePlayerController (Game|GetPlayerController 0)))
  (Variables|Default|SetPlayer%20Jam%20Controller _asscore_player_controller)
  (Class|EventsManager|SpawnEvent))

(event Collision|EventActorBeginOverlap
  (params (OtherActor :type Actor%20Object%20Reference)))

(event EventTick
  (params (DeltaSeconds :type Float%20%28single-precision%29)))

(event EventShowRewardsUI
  (bind _returnvalue (UserInterface|CreateWidget "/Game/Blueprints/Widgets/BP_EventRewards.BP_EventRewards_C" (Game|GetPlayerController 0)))
  (bind _output_get (Variables|Default|SetEvent%20Rewards _returnvalue))
  (UserInterface|Viewport|AddtoViewport _output_get 0)
  (Variables|/Script/Engine.PlayerController|SetbShowMouseCursor (Variables|Default|GetPlayer%20Jam%20Controller) true))

(event EventSwitchEventUI
  (bind _player_jam_controller (Variables|Default|GetPlayer%20Jam%20Controller))
  (bind _player_ui (Variables|/Game/Blueprints/ScorePlayerController.ScorePlayerController_C|GetPlayer%20UI _player_jam_controller))
  (bind _eventtimer (Variables|/Game/Blueprints/Widgets/BP_PlayerUIWidget.BP_PlayerUIWidget_C|GetEventTImer _player_ui))
  (if (Widget|IsVisible (Variables|/Game/Blueprints/Widgets/BP_PlayerUIWidget.BP_PlayerUIWidget_C|GetEventTImer (Variables|/Game/Blueprints/ScorePlayerController.ScorePlayerController_C|GetPlayer%20UI (Variables|Default|GetPlayer%20Jam%20Controller))))
    (Variables|/Script/UMG.Widget|SetVisibility _eventtimer "Hidden")
    (else
      (Variables|/Script/UMG.Widget|SetVisibility _eventtimer "HitTestInvisible"))))

(fn ConstructionScript)