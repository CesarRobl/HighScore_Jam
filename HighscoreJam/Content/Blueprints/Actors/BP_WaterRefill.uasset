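; BP_WaterRefill is a zone actor that refills the shark player's water while the player is inside it.
; BeginPlay caches the first player character as a BP_SharkPlayer.
; Overlaps on the Cube component set and clear a CanRefill flag, and Tick calls RefillWater on the cached player every frame while it is set.
; Leaving the cube also sets the player's refill state to false.
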(event OnComponentBeginOverlap(Cube)
  (params (OverlappedComponent :type Primitive%20Component%20Object%20Reference) (OtherActor :type Actor%20Object%20Reference) (OtherComp :type Primitive%20Component%20Object%20Reference) (OtherBodyIndex :type Integer) (bFromSweep :type Boolean) (SweepResult :type Hit%20Result%20Structure%20%28by%20ref%29))
  (Utilities|Casting|CastToBP_SharkPlayer OtherActor)
  (Variables|Default|SetCanRefill true))

(event OnComponentEndOverlap(Cube)
  (params (OverlappedComponent :type Primitive%20Component%20Object%20Reference) (OtherActor :type Actor%20Object%20Reference) (OtherComp :type Primitive%20Component%20Object%20Reference) (OtherBodyIndex :type Integer))
  (Utilities|Casting|CastToBP_SharkPlayer OtherActor)
  (Variables|Default|SetCanRefill false)
  (Class|HighscoreJamCharacter|SetRefillState (Variables|Default|GetPlayer) false))

(event EventBeginPlay
  (bind _asbp_shark_player (Utilities|Casting|CastToBP_SharkPlayer (Game|GetPlayerCharacter 0)))
  (Variables|Default|SetPlayer _asbp_shark_player))

(event Collision|EventActorBeginOverlap
  (params (OtherActor :type Actor%20Object%20Reference)))

(event EventTick
  (params (DeltaSeconds :type Float%20%28single-precision%29))
  (if (Variables|Default|GetCanRefill)
    (Class|HighscoreJamCharacter|RefillWater (Variables|Default|GetPlayer))))

(fn ConstructionScript)