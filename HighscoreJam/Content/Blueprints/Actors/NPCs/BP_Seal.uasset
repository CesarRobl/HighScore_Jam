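; BP_Seal is an NPC Blueprint that builds rage and charges at its target character.
; UseAbility accumulates delta time into Rage; past the threshold it locks a charge location and raises walk speed until an attack resets rage.
; GetTargetPosition skips the parent's targeting while charging.
; The random unit offset around the target feeds a radian-range angle into degree-based trig, so its direction barely varies.
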(event EventBeginPlay
  (|CallParentFunction) ; This node is disabled and will not be called.\nDrag off pins to build functionality.
)

(event Collision|EventActorBeginOverlap
  (params (OtherActor :type Actor%20Object%20Reference)))

(event EventTick
  (params (DeltaSeconds :type Float%20%28single-precision%29))
  (|CallParentFunction DeltaSeconds) ; This node is disabled and will not be called.\nDrag off pins to build functionality.
)

(event EventUseAbility
  (bind _output_get (Variables|Default|SetRage (+ (Variables|Default|GetRage) (Utilities|Time|GetWorldDeltaSeconds))))
  (if (> _output_get 1e+01)
    (CallFunction|OffsetLocation)
    (if (Variables|Default|GetbIsAttacking)
      (Variables|Default|SetRage 0.0)
      (Variables|Default|SetIsCharging false)
      (else
        (Variables|/Script/Engine.CharacterMovementComponent|SetMaxWalkSpeed (Variables|Character|GetCharacterMovement) 6e+02)))))

(fn ConstructionScript
  (|CallParentFunction))

(fn OffsetLocation
  (if (not (Variables|Default|GetIsCharging))
    (LocalVariables|SetAngle (Math|Random|RandomFloatinRange 0.0 (Math|Float|MultiplybyPi 2.0)))
    (bind _output_get (LocalVariables|SetOffset (Math|Vector|MakeVector (Math|Trig|Cos(Degrees) (LocalVariables|GetAngle)) (Math|Trig|Sin(Degrees) (LocalVariables|GetAngle)) 0.0)))
    (Variables|Default|SetTargetLocation (+ _output_get (Transformation|GetActorLocation (Variables|Default|GetTargetCharacter))))
    (Variables|Default|SetIsCharging true)))

(fn GetTargetPosition
  (if (not (Variables|Default|GetIsCharging))
    (|CallParentFunction)))