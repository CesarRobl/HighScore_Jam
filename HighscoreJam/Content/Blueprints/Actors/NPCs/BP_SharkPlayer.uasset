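; Player shark character Blueprint that handles shooting, shop interaction and death collision.
; IA_Shoot calls FireRay and Shoot while Water stat remains; FireRay capsule-traces from the actor along the view direction with debug drawing, casting hits to BP_BaseAI without further action.
; Mesh overlaps track the nearby BP_Shop, whose UI E opens.
; Tick disables capsule collision when dead.
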(event OnComponentBeginOverlap(Mesh)
  (params (OverlappedComponent :type Primitive%20Component%20Object%20Reference) (OtherActor :type Actor%20Object%20Reference) (OtherComp :type Primitive%20Component%20Object%20Reference) (OtherBodyIndex :type Integer) (bFromSweep :type Boolean) (SweepResult :type Hit%20Result%20Structure%20%28by%20ref%29))
  (bind _asbp_shop (Utilities|Casting|CastToBP_Shop OtherActor))
  (Variables|Default|SetAs%20BP%20Shop _asbp_shop))

(event OnComponentEndOverlap(Mesh)
  (params (OverlappedComponent :type Primitive%20Component%20Object%20Reference) (OtherActor :type Actor%20Object%20Reference) (OtherComp :type Primitive%20Component%20Object%20Reference) (OtherBodyIndex :type Integer))
  (Utilities|Casting|CastToBP_Shop OtherActor)
  (Variables|Default|SetAs%20BP%20Shop 0))

(event Input|EnhancedActionEvents|EnhancedInputActionIA_Shoot
  (params (ActionValue :type Boolean) (ElapsedSeconds :type Float%20%28double-precision%29) (TriggeredSeconds :type Float%20%28double-precision%29) (InputAction :type Input%20Action%20Object%20Reference :default "/Game/Inputs/Actions/IA_Shoot.IA_Shoot"))
  (:Triggered
    (if (not (<= (.water (Variables|Default|GetPlayerStats)) 0.0)) :!label _label
      (CallFunction|FireRay)
      (Class|HighscoreJamCharacter|Shoot)))
  (:Ongoing
    (goto _label)))

(event EventBeginPlay)

(event Collision|EventActorBeginOverlap
  (params (OtherActor :type Actor%20Object%20Reference)))

(event EventTick
  (params (DeltaSeconds :type Float%20%28single-precision%29))
  (if (Class|HighscoreJamCharacter|IsDead)
    (Collision|SetCollisionEnabled (Variables|Default|GetCapsuleComponent) "NoCollision")))

(event Input|KeyboardEvents|E
  (params (Key :type Key%20Structure :default "None"))
  (bind _as_bp_shop (Variables|Default|GetAs%20BP%20Shop))
  (:Pressed
    (Utilities|IsValid _as_bp_shop
      (:Is%20Valid
        (Default|ShopUI _as_bp_shop)))))

(fn ConstructionScript)

(fn FireRay
  (bind _returnvalue (Pawn|GetController))
  (bind _playerstats (Variables|Default|GetPlayerStats))
  (bind (_location _rotation) (Pawn|GetPlayerViewPoint _returnvalue))
  (bind _outhit (Collision|CapsuleTraceByChannel (Transformation|GetActorLocation) (+ _location (* _rotation 1e+04)) (.capsuleradius _playerstats) (.capsulehalfheight _playerstats) "TraceTypeQuery1" false 0 "ForOneFrame"))
  (Utilities|Casting|CastToBP_BaseAI (.hitactor _outhit)))