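; BP_Seagull is an NPC that makes ranged attacks on a target character.
; PerformAttack spawns a BP_ProjectileBase at the seagull's transform and launches it at a fixed speed along the normalized direction to TargetCharacter's current location.
; The Blueprint contains no targeting or attack-timing logic, and its BeginPlay, overlap and Tick events are disabled stubs.
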(event EventBeginPlay
  (|CallParentFunction) ; This node is disabled and will not be called.\nDrag off pins to build functionality.
)

(event Collision|EventActorBeginOverlap
  (params (OtherActor :type Actor%20Object%20Reference)))

(event EventTick
  (params (DeltaSeconds :type Float%20%28single-precision%29))
  (|CallParentFunction DeltaSeconds) ; This node is disabled and will not be called.\nDrag off pins to build functionality.
)

(event EventPerformAttack
  (bind _returnvalue (Game|SpawnActorfromClass "/Game/Blueprints/Actors/BP_ProjectileBase.BP_ProjectileBase_C" (Transformation|GetActorTransform) "Undefined" "MultiplyWithRoot" 0 0))
  (Default|ShootProjectile _returnvalue (Math|Vector|Normalize (- (Transformation|GetActorLocation (Variables|Default|GetTargetCharacter)) (Transformation|GetActorLocation))) 1.7e+03))

(fn ConstructionScript
  (|CallParentFunction))